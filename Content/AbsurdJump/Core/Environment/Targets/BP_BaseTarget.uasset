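; BP_BaseTarget is a shootable target that grants the player a reward when damaged, then destroys itself.
; On BeginPlay it labels its TextRender with its TargetType name.
; On the first damage event it plays a hit sound, then switches on TargetType: Boost boosts the player character, Ammo gives ammo through its EquipmentComponent.
; Both types also add score.
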(event Custom|Damaged
  (Utilities|FlowControl|DoOnce false
    (:Completed
      (bind _asbp_character (Utilities|Casting|CastToBP_Character (Game|GetPlayerCharacter 0)))
      (Audio|SpawnSoundatLocation "/Game/AbsurdJump/Audio/SFX/Sounds/S_BoostButtonHit.S_BoostButtonHit" (Transformation|GetWorldLocation (Variables|Default|GetDefaultSceneRoot)) "0, 0, 0" 1.0 1.0 0.0 0 0)
      (switch Utilities|FlowControl|Switch|SwitchonE_TargetType (Variables|Default|GetTargetType)
        (:NewEnumerator1
          (Class|AJCharacterBase|Boost _asbp_character)
          (Class|AJCharacterBase|AddScore _asbp_character 10))
        (:NewEnumerator2
          (Class|AJCharacterEquipmentComponent|GiveAmmo (Variables|/Script/AbsurdJump.AJ_CharacterBase|GetEquipmentComponent _asbp_character) (Variables|Ammo|GetAmmoToGive))
          (Class|AJCharacterBase|AddScore _asbp_character 5)))
      (Actor|DestroyActor))))

(event EventBeginPlay
  (Rendering|Components|TextRender|SetText (Variables|Default|GetTextRender) (Utilities|Text|ToText(String) (Utilities|String|EnumtoString (Variables|Default|GetTargetType)))))

(event Collision|EventActorBeginOverlap
  (params (OtherActor :type Actor%20Object%20Reference)))

(event EventTick
  (params (DeltaSeconds :type Float%20%28single-precision%29)))

(fn ConstructionScript)