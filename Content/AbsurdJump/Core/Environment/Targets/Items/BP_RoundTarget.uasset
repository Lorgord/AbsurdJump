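; BP_RoundTarget is a round target that labels itself with its target type and spins when damaged.
; On BeginPlay it writes the TargetType enum name to its TextRender.
; Damaged plays the TargetRotation timeline, which sets the mesh's world roll, with IsInversed choosing the direction, and calls Damaged on each update.
; A hit-sound branch is present but disconnected, so it never runs.
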(event EventBeginPlay
  (Rendering|Components|TextRender|SetText (Variables|Default|GetTextRender) (Utilities|Text|ToText(String) (Utilities|String|EnumtoString (Variables|Default|GetTargetType)))))

(event EventDamaged
  (bind _rotation (Timeline|TargetRotation Play)
    (:Update
      (if (Variables|Default|GetbIsInversed)
        (Transformation|SetWorldRotation (Variables|Default|GetStaticMesh) (Math|Rotator|MakeRotator (.x _rotation) 0.0 0.0) false false)
        (else
          (Transformation|SetWorldRotation (Variables|Default|GetStaticMesh) (Math|Rotator|MakeRotator (* (.x _rotation) -1.0) 0.0 0.0) false false)))
      (CallFunction|Damaged))))

(fn ConstructionScript)